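; Game mode for a game jam project that handles the end-of-game sequence and tracks how many people were accepted.
; Once all characters have spawned, BWon clears HUD widgets, fades the score and writes a reflection chosen by the accepted count.
; The Delaying event does not pause BWon, so the score is removed immediately.
; Tick can dim the directional light; ToCredits creates the credits widget, then returns to the main menu.
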(event `self.ReceiveBeginPlay`
  (`|ExecutionSequence`
    (:`then_0`
      (bind _returnvalue (`GameplayStatics.GetActorOfClass` "/Game/BP_HUD.BP_HUD_C"))
      (set `self.BP_HUD` _returnvalue))
    (:`then_1`
      (bind _returnvalue_2 (`GameplayStatics.GetActorOfClass` "/Script/Engine.DirectionalLight"))
      (set `self.Luzdirectional` _returnvalue_2))
    (:`then_2`
      (set `self.Order` 1))))

(event `self.ReceiveTick`
  (params (DeltaSeconds :type "Float (single-precision)"))
  (if (`self.Turn lights`)
    (`LightComponent.SetIntensity` (`Light.LightComponent` (`self.Luzdirectional`)) (`KismetMathLibrary.FInterpTo` (`LightComponentBase.Intensity` (`Light.LightComponent` (`self.Luzdirectional`))) 0.0 DeltaSeconds (`self.DuracionApagado`)))))

(event `Delaying`
  (`KismetSystemLibrary.Delay` 8.0))

(event `/Game/InterfacesNotUI/ToCredits.ToCredits`
  (params (ToCredits :type Boolean))
  (`Widget.RemoveFromParent` (`/Game/BP_HUD.Reflection` (`self.BP_HUD`)))
  (bind _returnvalue (`|CreateWidget` "/Game/UserInterface/WBP_Credits.WBP_Credits_C" (`GameplayStatics.GetPlayerController` 0)))
  (set `self.Credits` _returnvalue)
  (`KismetSystemLibrary.Delay` 10.0)
  (`GameplayStatics.OpenLevel` "Level_MainMenu"))

(fn `AddingAccepted`
  (set `self.PeopleAccepted` (+ (`self.PeopleAccepted`) 1)))

(fn `B Won`
  (params (AllCharactersAlreadySpawned :type Boolean))
  (bind _bp_hud (`self.BP_HUD`))
  (bind _score (`/Game/BP_HUD.Score` _bp_hud))
  (bind _reflection (`/Game/BP_HUD.Reflection` (`self.BP_HUD`)))
  (if AllCharactersAlreadySpawned
    (for _array_element (`/Game/BP_HUD.GamesWidgets` _bp_hud)
      (`Widget.RemoveFromParent` _array_element))
    (for _array_element_2 (`/Game/BP_HUD.Menu&Options` _bp_hud)
      (`Widget.RemoveFromParent` _array_element_2))
    (for _array_element_3 (`/Game/BP_HUD.InteractiveUI` _bp_hud)
      (`Widget.RemoveFromParent` _array_element_3))
    (`UserWidget.AddToViewport` _score 0)
    (`/Game/UserInterface/WBP_PlayerScore.Fade` _score)
    (`self.Delaying`)
    (`Widget.RemoveFromParent` _score)
    (`UserWidget.AddToViewport` _reflection 0)
    (if (>= (`self.PeopleAccepted`) 5)
      (set `/Game/UserInterface/WBP_Reflection.FullText` (`self.Reflexion`) _reflection)
      (else
        (set `/Game/UserInterface/WBP_Reflection.FullText` (`self.ReflexinNonGood`) _reflection)))
    (`/Game/UserInterface/WBP_Reflection.WriteEnd` _reflection)))

(fn `UserConstructionScript`)